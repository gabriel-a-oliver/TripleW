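; BP_BurstRifle is a child weapon Blueprint that rate-limits the firing behavior it inherits from its parent.
; The construction script sets the fire delay, and Tick counts a cooldown timer down by world delta seconds.
; The FireWeapon override calls the parent's fire logic only when that timer has run out, restarting the cooldown each time.
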(event `self.ReceiveTick`
  (params (DeltaSeconds :type "Float (single-precision)"))
  (set `self.FireWeaponTimer` (- (`self.FireWeaponTimer`) (`GameplayStatics.GetWorldDeltaSeconds`))))

(fn `FireWeapon`
  (if (<= (`self.FireWeaponTimer`) 0.0)
    (set `self.FireWeaponTimer` (`self.FireWeaponDelay`))
    (`parent.FireWeapon`)))

(fn `UserConstructionScript`
  (`parent.UserConstructionScript`)
  (set `self.FireWeaponDelay` 0.5))