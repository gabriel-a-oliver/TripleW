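; BPC_AutomaticWeapon is a firing-mode component that configures its owning BP_Gun for automatic fire.
; On BeginPlay it casts its owner to BP_Gun, copies its local fire delay to the gun, disables burst and single modes, and sets the fire mode enum.
; A failed cast prints an error message, which still names the single-fire component.
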(event `self.ReceiveBeginPlay`
  (bind _ownerreference (`self.OwnerReference`))
  (bind _output_get (set `self.OwnerGun` (`self.GetOwner`)))
  (bind _asbp_gun (cast `/Game/Blueprints/Weapons/BP_Gun` _output_get)
    (:`then`
      (set `self.OwnerReference` _asbp_gun)
      (set `/Game/Blueprints/Weapons/BP_Gun.FireWeaponDelay` (`self.LocalFireWeaponDelay`) _ownerreference)
      (set `/Game/Blueprints/Weapons/BP_Gun.BurstEnabled` false _ownerreference)
      (set `/Game/Blueprints/Weapons/BP_Gun.SingleEnabled` false _ownerreference)
      (set `/Game/Blueprints/Weapons/BP_Gun.WeaponFireMode` "NewEnumerator2" _ownerreference))
    (:`CastFailed`
      (`KismetSystemLibrary.PrintString` "Cast Failed: Single Fire Component"))))