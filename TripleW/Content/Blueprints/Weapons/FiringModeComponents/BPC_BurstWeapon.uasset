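; BPC_BurstWeapon is a firing-mode component that configures its owning BP_Gun as a burst weapon.
; On BeginPlay it casts the owner to BP_Gun, pushes its local fire delay, shots per burst and in-burst delay, disables single and automatic fire, and sets the fire mode enum.
; It holds no firing logic in this graph, and prints an error if the owner is not a BP_Gun.
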(event `self.ReceiveBeginPlay`
  (bind _ownerreference (`self.OwnerReference`))
  (bind _output_get (set `self.OwnerGun` (`self.GetOwner`)))
  (bind _asbp_gun (cast `/Game/Blueprints/Weapons/BP_Gun` _output_get)
    (:`then`
      (set `self.OwnerReference` _asbp_gun)
      (set `/Game/Blueprints/Weapons/BP_Gun.FireWeaponDelay` (`self.LocalFireWeaponDelay`) _ownerreference)
      (set `/Game/Blueprints/Weapons/BP_Gun.SingleEnabled` false _ownerreference)
      (set `/Game/Blueprints/Weapons/BP_Gun.AutomaticEnabled` false _ownerreference)
      (set `/Game/Blueprints/Weapons/BP_Gun.FiresPerBurst` (`self.LocalNumberOfShots`) _ownerreference)
      (set `/Game/Blueprints/Weapons/BP_Gun.BurstDelayBetweenShots` (`self.LocalBurstDelayBetweenShots`) _ownerreference)
      (set `/Game/Blueprints/Weapons/BP_Gun.WeaponFireMode` "NewEnumerator1" _ownerreference))
    (:`CastFailed`
      (`KismetSystemLibrary.PrintString` "Cast Failed: Burst Component"))))