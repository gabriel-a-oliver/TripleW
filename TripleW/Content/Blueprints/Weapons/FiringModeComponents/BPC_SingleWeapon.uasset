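; BPC_SingleWeapon is a firing mode component that configures its owning BP_Gun for single fire.
; On BeginPlay it casts its owner to BP_Gun, applies its local fire delay, turns off burst and automatic firing, and sets the gun's fire mode enum.
; If the owner is not a BP_Gun, it prints a cast failure message.
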(event `self.ReceiveBeginPlay`
  (bind _owner_reference (`self.Owner Reference`))
  (bind _output_get (set `self.Owner Gun` (`self.GetOwner`)))
  (bind _asbp_gun (cast `/Game/Blueprints/Weapons/BP_Gun` _output_get)
    (:`then`
      (set `self.Owner Reference` _asbp_gun)
      (set `/Game/Blueprints/Weapons/BP_Gun.FireWeaponDelay` (`self.LocalFireWeaponDelay`) _owner_reference)
      (set `/Game/Blueprints/Weapons/BP_Gun.BurstEnabled` false _owner_reference)
      (set `/Game/Blueprints/Weapons/BP_Gun.AutomaticEnabled` false _owner_reference)
      (set `/Game/Blueprints/Weapons/BP_Gun.WeaponFireMode` "NewEnumerator0" _owner_reference))
    (:`CastFailed`
      (`KismetSystemLibrary.PrintString` "Cast Failed: Single Fire Component"))))